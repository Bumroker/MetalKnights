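; Enemy tank pawn that, when AutoAim is set, turns its turret toward player 0 every Tick.
; RotateForwardDirection (yaw toward a target) and RotateNewDirection (slower, to a given rotation) turn the actor through timeline-driven RInterpTo.
; The construction script applies EnemySpeed to FloatingPawnMovement.
; MovementRotation is an empty stub, and the cached player reference is flagged to change for multiplayer.
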(event `self.ReceiveBeginPlay`
  ;[1 0.7915 0] Cambiar Para El Multiplayer
  (`parent.ReceiveBeginPlay`)
  (set `self.Player` (`GameplayStatics.GetPlayerPawn` 0)))

(event `AutoAimActivation`
  (if (`self.AutoAim`)
    (`self.RotateTurret` (`self.K2_GetActorLocation` (`self.Player`)))))

(event `self.ReceiveTick`
  (params (DeltaSeconds :type "Float (single-precision)"))
  (`parent.ReceiveTick` DeltaSeconds)
  (`self.AutoAimActivation`)
  (`self.MovementRotation`))

(event `MovementRotation`)

(event `self.RotateForwardDirection`
  (params (LockAtTarget :type "Vector Structure"))
  (`Timeline|Timeline` :`NewTime` 0.5
    (:`Update`
      (`self.K2_SetActorRotation` (`KismetMathLibrary.RInterpTo` (`self.K2_GetActorRotation`) (`KismetMathLibrary.MakeRotator` 0.0 0.0 (.yaw (`KismetMathLibrary.Conv_VectorToRotator` (- LockAtTarget (`self.K2_GetActorLocation`))))) (`GameplayStatics.GetWorldDeltaSeconds`) 10.0)))))

(event `RotateNewDirection`
  (params (NewDirection :type "Rotator Structure"))
  (`Timeline|Timeline_0` :`NewTime` 0.4 :!via `PlayFromStart`
    (:`Update`
      (`self.K2_SetActorRotation` (`KismetMathLibrary.RInterpTo` (`self.K2_GetActorRotation`) NewDirection (`GameplayStatics.GetWorldDeltaSeconds`) 0.4)))))

(fn `UserConstructionScript`
  (`parent.UserConstructionScript`)
  (set `FloatingPawnMovement.MaxSpeed` (`self.Enemy_Speed`) (`self.FloatingPawnMovement`)))