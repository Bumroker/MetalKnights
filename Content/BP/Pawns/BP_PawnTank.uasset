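; Tank pawn Blueprint that provides tank-style movement: driving along its local forward axis and turning in yaw.
; Navigation takes a two-axis input, using X for a swept local move and Y for an unswept local rotation.
; CalculateSpeed scales each axis by its speed and world delta time, with a Slow divisor left neutral.
; The event graph is empty, so nothing here calls Navigation.
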(event `self.ReceiveBeginPlay`)

(fn `CalculateSpeed`
  (params (Direction :type "Float (double-precision)") (MovementSpeed :type "Float (double-precision)") (Slow :type "Float (double-precision)" :default 1.0))
  (returns (Speed :type "Float (double-precision)"))
  (return (/ (* Direction MovementSpeed (`GameplayStatics.GetWorldDeltaSeconds`)) Slow)))

(fn `Navigation`
  (params (Navigation :type "Vector2D Structure"))
  (bind (_x _y) (`KismetMathLibrary.BreakVector2D` Navigation))
  (`self.K2_AddActorLocalOffset` (`KismetMathLibrary.MakeVector` (`self.CalculateSpeed` _x (`self.MovementSpeed`))) true)
  (`self.K2_AddActorLocalRotation` (`KismetMathLibrary.MakeRotator` 0.0 0.0 (`self.CalculateSpeed` _y (`self.RotationSpeed`)))))

(fn `UserConstructionScript`)