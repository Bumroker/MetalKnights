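; BP_Tank is a tank Blueprint, filed under Unused pawns, that moves with tank-style forward and turn controls.
; Navigation maps the input's X to a local forward offset and Y to local yaw, both without sweep.
; CalculateSpeed scales each axis by Speed and world delta time, with turning divided down to half rate.
; Its events and construction script only call the parent.
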(event `self.ReceiveBeginPlay`
  (`parent.ReceiveBeginPlay`))

(event `self.ReceiveActorBeginOverlap`
  (params (OtherActor :type "Actor Object Reference"))
  (`parent.ReceiveActorBeginOverlap` OtherActor))

(event `self.ReceiveTick`
  (params (DeltaSeconds :type "Float (single-precision)"))
  (`parent.ReceiveTick` DeltaSeconds))

(fn `CalculateSpeed`
  (params (Direction :type "Float (double-precision)") (Slow :type "Float (double-precision)" :default 1.0))
  (returns (Speed :type "Float (double-precision)"))
  (return (/ (* Direction (`self.Speed`) (`GameplayStatics.GetWorldDeltaSeconds`)) Slow)))

(fn `Navigation`
  (params (Navigation :type "Vector2D Structure"))
  (bind (_x _y) (`KismetMathLibrary.BreakVector2D` Navigation))
  (`self.K2_AddActorLocalOffset` (`KismetMathLibrary.MakeVector` (`self.CalculateSpeed` _x)))
  (`self.K2_AddActorLocalRotation` (`KismetMathLibrary.MakeRotator` 0.0 0.0 (`self.CalculateSpeed` _y 2.0))))

(fn `UserConstructionScript`
  (`parent.UserConstructionScript`))