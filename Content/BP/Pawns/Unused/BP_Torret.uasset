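; BP_Torret is a turret Blueprint, filed under unused pawns, that turns to track the player.
; It caches the first player pawn on BeginPlay and passes that pawn's location to RotateTurret every Tick, with no validity check.
; RotateTurret is not defined in this graph, and the overlap event and construction script only forward to the parent class.
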(event `self.ReceiveBeginPlay`
  (`parent.ReceiveBeginPlay`)
  (set `self.Player` (`GameplayStatics.GetPlayerPawn` 0)))

(event `self.ReceiveActorBeginOverlap`
  (params (OtherActor :type "Actor Object Reference"))
  (`parent.ReceiveActorBeginOverlap` OtherActor))

(event `self.ReceiveTick`
  (params (DeltaSeconds :type "Float (single-precision)"))
  (`parent.ReceiveTick` DeltaSeconds)
  (`self.RotateTurret` (`self.K2_GetActorLocation` (`self.Player`))))

(fn `UserConstructionScript`
  (`parent.UserConstructionScript`))