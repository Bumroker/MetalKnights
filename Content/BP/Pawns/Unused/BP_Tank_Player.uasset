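; Player-controlled tank pawn, stored in an Unused folder, that drives and fires through Enhanced Input and aims at the mouse cursor.
; BeginPlay adds the input mapping context, and the shoot and navigation actions call Fire and Navigation, which are not defined here.
; Every Tick, the Shoot function only aims, despite its name, passing the under-cursor Visibility trace impact point to RotateTurret.
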(event `self.ReceiveBeginPlay`
  (`parent.ReceiveBeginPlay`)
  (bind _asplayer_controller (cast `PlayerController` (`self.GetController`)))
  (bind _returnvalue (pcsubsystem `EnhancedInputLocalPlayerSubsystem` _asplayer_controller))
  (`/Engine/EditorBlueprintResources/StandardMacros.IsValid` _returnvalue
    (:`Is Valid`
      (`EnhancedInputSubsystemInterface.AddMappingContext` _returnvalue "/Game/BP/Input/MyGameInputMapping.MyGameInputMapping" 0 (struct)))))

(event `EnhancedInput|/Game/BP/Input/IA_Shoot`
  (params (ActionValue :type Boolean) (ElapsedSeconds :type "Float (double-precision)") (TriggeredSeconds :type "Float (double-precision)") (InputAction :type "InputAction Object Reference" :default "/Game/BP/Input/IA_Shoot.IA_Shoot"))
  (:`Started`
    (`self.Fire`)))

(event `self.ReceiveTick`
  (params (DeltaSeconds :type "Float (single-precision)"))
  (`parent.ReceiveTick` DeltaSeconds)
  (`self.Shoot`))

(event `EnhancedInput|/Game/BP/Input/IA_Navigation`
  (params (ActionValue :type "Vector2D Structure") (ElapsedSeconds :type "Float (double-precision)") (TriggeredSeconds :type "Float (double-precision)") (InputAction :type "InputAction Object Reference" :default "/Game/BP/Input/IA_Navigation.IA_Navigation"))
  (:`Triggered`
    (`self.Navigation` ActionValue)))

(fn `Shoot`
  (`self.RotateTurret` (`.ImpactPoint` (`GameplayStatics.BreakHitResult` (`PlayerController.GetHitResultUnderCursorByChannel` (`GameplayStatics.GetPlayerController` 0) "TraceTypeQuery1" false)))))

(fn `UserConstructionScript`
  (`parent.UserConstructionScript`))