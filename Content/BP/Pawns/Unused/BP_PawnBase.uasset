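; Base pawn with base and turret meshes, set in the construction script, that can aim and fire.
; Fire spawns a self-owned BP_Proyectil at SpawnPoint.
; RotateTurret applies yaw-only rotation toward a target, using RInterpTo with the look-at rotation as Current and the turret's rotation as Target.
; HandleDestruction spawns an emitter and 2D sound, while TakeDmg and Death are empty stubs.
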(event `self.ReceiveBeginPlay`)

(fn `Death`)

(fn `Fire`
  (bind _returnvalue (`|SpawnActorFromClass` "/Game/BP/Actors/BP_Proyectil.BP_Proyectil_C" (`SceneComponent.K2_GetComponentToWorld` (`self.SpawnPoint`)) "Undefined" "OverrideRootScale" null null))
  (`self.SetOwner` _returnvalue self))

(fn `GetRotationFromTarget`
  (params (Target :type "Vector Structure"))
  (returns (NewRotation :type "Rotator Structure"))
  (bind _turret (`self.Turret`))
  (return (`KismetMathLibrary.RInterpTo` (`KismetMathLibrary.MakeRotator` 0.0 0.0 (+ (.yaw (`KismetMathLibrary.MakeRotFromZ` (- Target (`SceneComponent.K2_GetComponentLocation` _turret)))) -90.0)) (`SceneComponent.K2_GetComponentRotation` _turret) (`GameplayStatics.GetWorldDeltaSeconds`) 25.0)))

(fn `HandleDestruction`
  (`GameplayStatics.SpawnEmitterAtLocation` null (.location (`self.GetTransform`)) (.rotation (`self.GetTransform`)) (.scale (`self.GetTransform`)))
  (`GameplayStatics.SpawnSound2D` null 1.0 1.0 0.0 null))

(fn `RotateTurret`
  (params (LookAtTarget :type "Vector Structure"))
  (`SceneComponent.K2_SetWorldRotation` (`self.Turret`) (`self.GetRotationFromTarget` LookAtTarget) false false))

(fn `TakeDmg`)

(fn `UserConstructionScript`
  (`StaticMeshComponent.SetStaticMesh` (`self.Base`) (`self.BaseMesh`))
  (`StaticMeshComponent.SetStaticMesh` (`self.Turret`) (`self.TurretMesh`)))