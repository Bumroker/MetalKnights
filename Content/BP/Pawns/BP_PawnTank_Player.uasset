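; Player-controlled tank pawn that connects Enhanced Input to the tank's firing and navigation.
; On BeginPlay it runs parent logic, casts its controller to BP_TTPlayerController and adds the input mapping context to that player's subsystem.
; The shoot action calls Fire when started, and the navigation action passes its value to Navigation while triggered.
; Neither function is defined in this Blueprint's graphs.
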(event `self.ReceiveBeginPlay`
  (`parent.ReceiveBeginPlay`)
  (bind _asbp_ttplayer_controller (cast `/Game/BP/GameMode/BP_TTPlayerController` (`self.GetController`)))
  (bind _returnvalue (pcsubsystem `EnhancedInputLocalPlayerSubsystem` _asbp_ttplayer_controller))
  (`/Engine/EditorBlueprintResources/StandardMacros.IsValid` _returnvalue
    (:`Is Valid`
      (`EnhancedInputSubsystemInterface.AddMappingContext` _returnvalue "/Game/BP/GameMode/Input/MyGameInputMapping.MyGameInputMapping" 0 (struct)))))

(event `EnhancedInput|/Game/BP/GameMode/Input/IA_Shoot`
  (params (ActionValue :type Boolean) (ElapsedSeconds :type "Float (double-precision)") (TriggeredSeconds :type "Float (double-precision)") (InputAction :type "InputAction Object Reference" :default "/Game/BP/GameMode/Input/IA_Shoot.IA_Shoot"))
  (:`Started`
    (`self.Fire` false)))

(event `EnhancedInput|/Game/BP/GameMode/Input/IA_Navigation`
  (params (ActionValue :type "Vector2D Structure") (ElapsedSeconds :type "Float (double-precision)") (TriggeredSeconds :type "Float (double-precision)") (InputAction :type "InputAction Object Reference" :default "/Game/BP/GameMode/Input/IA_Navigation.IA_Navigation"))
  (:`Triggered`
    (`self.Navigation` ActionValue)))

(fn `UserConstructionScript`
  (`parent.UserConstructionScript`))