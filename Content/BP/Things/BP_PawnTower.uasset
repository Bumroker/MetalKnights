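; BP_PawnTower is a turret tower pawn that either aims at the player or pivots its turret.
; BeginPlay runs the parent logic and caches player pawn 0, which an author note flags to change for multiplayer.
; Each Tick calls AutoAimActivation, which passes the player's location to RotateTurret when AutoAim is set and calls PivotTurret otherwise.
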(event `self.ReceiveBeginPlay`
  ;[1 0.7915 0] Cambiar Para El Multiplayer
  (`parent.ReceiveBeginPlay`)
  (set `self.Player` (`GameplayStatics.GetPlayerPawn` 0)))

(event `self.ReceiveTick`
  (params (DeltaSeconds :type "Float (single-precision)"))
  (`self.AutoAimActivation`))

(event `AutoAimActivation`
  (if (`self.AutoAim`)
    (`self.RotateTurret` (`self.K2_GetActorLocation` (`self.Player`)))
    (else
      (`self.PivotTurret`))))

(fn `UserConstructionScript`)