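; Player-controlled tank pawn that builds on a parent class for turret rotation, firing, navigation and slip on collision.
; On begin play it snaps to a fixed height, and each tick it aims the turret at the point under the cursor.
; Enhanced Input drives movement and shooting while alive and unpaused, with shot bounce settings read from GameInstance debug options.
; The pause input toggles game pause with a DebugMenu widget.
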(event `self.ReceiveBeginPlay`
  (`parent.ReceiveBeginPlay`)
  (`self.K2_SetActorLocation` (`KismetMathLibrary.MakeVector` (.x (`self.K2_GetActorLocation`)) (.y (`self.K2_GetActorLocation`)) 50.0) false true))

(event `self.ReceiveTick`
  (params (DeltaSeconds :type "Float (single-precision)"))
  (`parent.ReceiveTick` DeltaSeconds)
  (`self.RotateTurret` (`.ImpactPoint` (`GameplayStatics.BreakHitResult` (`PlayerController.GetHitResultUnderCursorByChannel` (`GameplayStatics.GetPlayerController` 0) "TraceTypeQuery1" false)))))

(event `EnhancedInput|/Game/BP/GameMode/Input/Input_Shoot`
  (params (ActionValue :type Boolean) (ElapsedSeconds :type "Float (double-precision)") (TriggeredSeconds :type "Float (double-precision)") (InputAction :type "InputAction Object Reference" :default "/Game/BP/GameMode/Input/Input_Shoot.Input_Shoot"))
  (bind ((`Rebotes?_8_0DD3312945E0EC4A7BFFBBA3FDBDB568` _rebotes_) (`NRebotes_6_5C6F51734D9969516E46F1A2DD38B316` _nrebotes)) (break `/Game/BP/Organization/Structs/DebugOptions` (`/Game/BP/GameMode/TankGameInstance.DebugOptions` (`self.GameInstance`))))
  (:`Started`
    (if (and (`self.Alive`) (not (`GameplayStatics.IsGamePaused`)))
      (`self.Fire` _rebotes_ _nrebotes "Player"))))

(event `EnhancedInput|/Game/BP/GameMode/Input/Input_Navigation`
  (params (ActionValue :type "Vector2D Structure") (ElapsedSeconds :type "Float (double-precision)") (TriggeredSeconds :type "Float (double-precision)") (InputAction :type "InputAction Object Reference" :default "/Game/BP/GameMode/Input/Input_Navigation.Input_Navigation"))
  (:`Triggered`
    (if (and (`self.Alive`) (not (`GameplayStatics.IsGamePaused`)))
      (`self.Navigation` true ActionValue_X ActionValue_Y))))

(event `self.BoxComp.OnComponentHit`
  (params (HitComponent :type "PrimitiveComponent Object Reference") (OtherActor :type "Actor Object Reference") (OtherComp :type "PrimitiveComponent Object Reference") (NormalImpulse :type "Vector Structure") (Hit :type "HitResult Structure (by ref)"))
  (`self.Slip` Hit))

(event `EnhancedInput|/Game/BP/GameMode/Input/Input_Pause`
  (params (ActionValue :type Boolean) (ElapsedSeconds :type "Float (double-precision)") (TriggeredSeconds :type "Float (double-precision)") (InputAction :type "InputAction Object Reference" :default "/Game/BP/GameMode/Input/Input_Pause.Input_Pause"))
  (:`Started`
    (if (`self.Alive`)
      (if (`GameplayStatics.IsGamePaused`)
        (`/Game/BP/Widget/DebugMenu.Continue` (`self.DebugMenu`))
        (else
          (`GameplayStatics.SetGamePaused` true)
          (bind _returnvalue (`|CreateWidget` "/Game/BP/Widget/DebugMenu.DebugMenu_C"))
          (bind _output_get (set `self.DebugMenu` _returnvalue))
          (set `/Game/BP/Widget/DebugMenu.Player` self _output_get)
          (`UserWidget.AddToViewport` _returnvalue 0))))))

(fn `UserConstructionScript`
  (`parent.UserConstructionScript`))