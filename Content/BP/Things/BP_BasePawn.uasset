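; BP_BasePawn is a base pawn that provides movement along its local forward axis and yaw rotation.
; Its construction script caches the TankGameInstance.
; Navigation either scales directional inputs by movement and rotation speeds through CalculateSpeed, or applies manual values directly as local offsets.
; Translation always sweeps for collision, while rotation sweeps only in automatic mode.
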(event `self.ReceiveBeginPlay`)

(fn `Navigation`
  (params (AutomaticMovement :type Boolean :default true) (`Up/Down` :type "Float (double-precision)") (`Left/Right` :type "Float (double-precision)") (`Manual Up/Down` :type "Float (double-precision)") (`Manual Left/Right` :type "Float (double-precision)"))
  (if AutomaticMovement
    (`self.K2_AddActorLocalOffset` (`KismetMathLibrary.MakeVector` (`self.CalculateSpeed` `Up/Down` (`self.MovementSpeed`))) true)
    (`self.K2_AddActorLocalRotation` (`KismetMathLibrary.MakeRotator` 0.0 0.0 (`self.CalculateSpeed` `Left/Right` (`self.RotationSpeed`))) true)
    (else
      (`self.K2_AddActorLocalOffset` (`KismetMathLibrary.MakeVector` `Manual Up/Down`) true)
      (`self.K2_AddActorLocalRotation` (`KismetMathLibrary.MakeRotator` 0.0 0.0 `Manual Left/Right`)))))

(fn `UserConstructionScript`
  (set `self.GameInstance` (cast `/Game/BP/GameMode/TankGameInstance` (`GameplayStatics.GetGameInstance`) :!pure true)))