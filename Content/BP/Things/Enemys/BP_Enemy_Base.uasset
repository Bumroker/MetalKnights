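; Base Blueprint for turreted enemies that caches player pawn 0 on BeginPlay, flagged in a Spanish note to change for multiplayer.
; AutoAimActivation either turns the turret toward the player or sweeps it back and forth within a pivot threshold.
; Construction applies movement and rotation speeds and positions the pathfinder and line-trace points from the movement radius.
; A helper derives turn angle, duration and delay toward a target location.
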(event `self.ReceiveBeginPlay`
  ;[1 0.7915 0] Cambiar Para El Multiplayer
  (`parent.ReceiveBeginPlay`)
  (set `self.Player` (`GameplayStatics.GetPlayerPawn` 0)))

(event `AutoAimActivation`
  (if (`self.AutoAim`)
    (`self.FaceDirection` (`self.K2_GetActorLocation` (`self.Player`)) (`self.TurretMesh`))
    (else
      (`self.PivoteTurret`))))

(event `self.ReceiveTick`
  (params (DeltaSeconds :type "Float (single-precision)"))
  (`parent.ReceiveTick` DeltaSeconds))

(fn `CalculateRotationDelay`
  (params (NewLocation :type "Vector Structure"))
  (returns (Angle :type "Float (double-precision)") (SecondsToRotate :type "Float (double-precision)") (RotaionDelay :type "Float (double-precision)"))
  (locals (BaseRotationDelay :type "Float (double-precision)" :default 0.2))
  (bind _yaw (.yaw (`KismetMathLibrary.FindRelativeLookAtRotation` (`self.GetTransform`) NewLocation)))
  (bind _returnvalue (/ (`KismetMathLibrary.Abs` _yaw) (`self.Enemy_RotationSpeed`)))
  (return _yaw _returnvalue (+ _returnvalue (`local.BaseRotationDelay`))))

(fn `PivoteTurret`
  (locals (PivoteThreshold :type "Float (double-precision)" :default 45.0) (LocalRotateTurretDirection :type "Float (double-precision)" :default 1.0) (ActualRotation :type Integer))
  (bind _pivotethreshold (`local.PivoteThreshold`))
  (bind _output_get (set `local.ActualRotation` (`KismetMathLibrary.FCeil` (.yaw (`SceneComponent.RelativeRotation` (`self.TurretMesh`))))))
  (if (<= _output_get (`KismetMathLibrary.FCeil` (* _pivotethreshold -1.0)))
    (set `self.BPRotateDirection` (`local.LocalRotateTurretDirection`))
    (elif (>= _output_get (`KismetMathLibrary.FCeil` _pivotethreshold))
      (set `self.BPRotateDirection` (* (`local.LocalRotateTurretDirection`) -1.0))))
  (`SceneComponent.K2_AddRelativeRotation` (`self.TurretMesh`) (`KismetMathLibrary.MakeRotator` 0.0 0.0 (`self.CalculateSpeed` (`self.BPRotateDirection`) (`self.RotationSpeed`) 8.0)) false false))

(fn `UserConstructionScript`
  (`parent.UserConstructionScript`)
  (set `FloatingPawnMovement.MaxSpeed` (`self.Enemy_Speed`) (`self.FloatingPawnMovement`))
  (set `self.RotationSpeed` (`self.Enemy_RotationSpeed`))
  (`SceneComponent.K2_SetRelativeLocation` (`self.PathFinderPoint`) (`KismetMathLibrary.MakeVector` (* (`self.MovementRadius`) 0.75)) true true)
  (`SceneComponent.K2_SetRelativeLocation` (`self.LineTraceEndPoint`) (`KismetMathLibrary.MakeVector` (- (.x (`SceneComponent.RelativeLocation` (`self.PathFinderPoint`))) (/ (`self.MovementRadius`) 3.0))) true true))