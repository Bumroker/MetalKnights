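; Player-controlled tank pawn that handles Enhanced Input for driving, shooting and pausing.
; BeginPlay adds the input mapping context for its player controller.
; While alive and unpaused, input feeds Navigation and Fire, with shots tagged "Player" and their bounce settings read from the GameInstance debug options.
; The pause input, also gated on being alive, pauses the game and opens a DebugMenu widget, or calls its Continue when already paused.
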(event `self.ReceiveBeginPlay`
  (`parent.ReceiveBeginPlay`)
  (bind _asbp_ttplayer_controller (cast `/Game/BP/GameMode/BP_TTPlayerController` (`self.GetController`)))
  (bind _returnvalue (pcsubsystem `EnhancedInputLocalPlayerSubsystem` _asbp_ttplayer_controller))
  (`/Engine/EditorBlueprintResources/StandardMacros.IsValid` _returnvalue
    (:`Is Valid`
      (`EnhancedInputSubsystemInterface.AddMappingContext` _returnvalue "/Game/BP/GameMode/Input/MyGameInputMapping.MyGameInputMapping" 0 (struct)))))

(event `EnhancedInput|/Game/BP/GameMode/Input/Input_Shoot`
  (params (ActionValue :type Boolean) (ElapsedSeconds :type "Float (double-precision)") (TriggeredSeconds :type "Float (double-precision)") (InputAction :type "InputAction Object Reference" :default "/Game/BP/GameMode/Input/Input_Shoot.Input_Shoot"))
  (bind ((`Rebotes?_8_0DD3312945E0EC4A7BFFBBA3FDBDB568` _rebotes_) (`NRebotes_6_5C6F51734D9969516E46F1A2DD38B316` _nrebotes)) (break `/Game/BP/Organization/Structs/DebugOptions` (`/Game/BP/GameMode/TankGameInstance.DebugOptions` (`self.GameInstance`))))
  (:`Started`
    (if (and (`self.Alive`) (not (`GameplayStatics.IsGamePaused`)))
      (`self.Fire` _rebotes_ _nrebotes "Player"))))

(event `EnhancedInput|/Game/BP/GameMode/Input/Input_Navigation`
  (params (ActionValue :type "Vector2D Structure") (ElapsedSeconds :type "Float (double-precision)") (TriggeredSeconds :type "Float (double-precision)") (InputAction :type "InputAction Object Reference" :default "/Game/BP/GameMode/Input/Input_Navigation.Input_Navigation"))
  (:`Triggered`
    (if (and (`self.Alive`) (not (`GameplayStatics.IsGamePaused`)))
      (`self.Navigation` true ActionValue_X ActionValue_Y))))

(event `EnhancedInput|/Game/BP/GameMode/Input/Input_Pause`
  (params (ActionValue :type Boolean) (ElapsedSeconds :type "Float (double-precision)") (TriggeredSeconds :type "Float (double-precision)") (InputAction :type "InputAction Object Reference" :default "/Game/BP/GameMode/Input/Input_Pause.Input_Pause"))
  (:`Started`
    (if (`self.Alive`)
      (if (`GameplayStatics.IsGamePaused`)
        (`/Game/BP/Widget/DebugMenu.Continue` (`self.DebugMenu`))
        (else
          (`GameplayStatics.SetGamePaused` true)
          (bind _returnvalue (`|CreateWidget` "/Game/BP/Widget/DebugMenu.DebugMenu_C"))
          (bind _output_get (set `self.DebugMenu` _returnvalue))
          (set `/Game/BP/Widget/DebugMenu.Player` self _output_get)
          (`UserWidget.AddToViewport` _returnvalue 0))))))

(fn `UserConstructionScript`
  (`parent.UserConstructionScript`))