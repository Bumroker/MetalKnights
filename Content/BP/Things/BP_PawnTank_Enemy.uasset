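; Enemy tank pawn that aims at or sweeps for the player, built on a parent that supplies turret and navigation functions.
; Construction applies enemy movement and rotation speeds; BeginPlay caches player 0, marked to change for multiplayer.
; Each tick, AutoAim chooses between tracking the player and pivoting the turret, while Rotate optionally steers the body through Navigation.
; The uncalled Blueprint pivot function, which bounces yaw between thresholds, is labeled as ported to C++.
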(event `self.ReceiveBeginPlay`
  ;[1 0.7915 0] Cambiar Para El Multiplayer
  (`parent.ReceiveBeginPlay`)
  (set `self.Player` (`GameplayStatics.GetPlayerPawn` 0)))

(event `AutoAimActivation`
  (if (`self.AutoAim`)
    (`self.RotateTurret` (`self.K2_GetActorLocation` (`self.Player`)))
    (else
      (`self.PivotTurret`))))

(event `self.ReceiveTick`
  (params (DeltaSeconds :type "Float (single-precision)"))
  (`parent.ReceiveTick` DeltaSeconds)
  (`self.AutoAimActivation`)
  (`self.MovementRotation`))

(event `MovementRotation`
  (if (`self.Rotate`)
    (`self.Navigation` true 0.0 (`self.BPRotateDirection`))))

(fn `BPPivoteTurret(traspasado a C++)`
  (locals (PivoteThreshold :type "Float (double-precision)" :default 45.0) (LocalRotateTurretDirection :type "Float (double-precision)" :default 1.0))
  (bind _pivotethreshold (`local.PivoteThreshold`))
  (bind _returnvalue (`KismetMathLibrary.FCeil` (.yaw (`SceneComponent.RelativeRotation` (`self.TurretMesh`)))))
  (if (<= _returnvalue (`KismetMathLibrary.FCeil` (* _pivotethreshold -1.0)))
    (set `self.BPRotateDirection` (`local.LocalRotateTurretDirection`))
    (elif (>= _returnvalue (`KismetMathLibrary.FCeil` _pivotethreshold))
      (set `self.BPRotateDirection` (* (`local.LocalRotateTurretDirection`) -1.0))))
  (`SceneComponent.K2_AddRelativeRotation` (`self.TurretMesh`) (`KismetMathLibrary.MakeRotator` 0.0 0.0 (`self.CalculateSpeed` (`self.BPRotateDirection`) (`self.RotationSpeed`) 8.0)) false false))

(fn `UserConstructionScript`
  (`parent.UserConstructionScript`)
  (set `FloatingPawnMovement.MaxSpeed` (`self.Enemy_Speed`) (`self.FloatingPawnMovement`))
  (set `self.RotationSpeed` (`self.Enemy_RotationSpeed`)))