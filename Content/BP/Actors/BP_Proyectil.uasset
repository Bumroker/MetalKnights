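; BP_Proyectil is a projectile actor that flies straight ahead and damages what it hits.
; Tick moves it along local X at Speed with a swept offset, and the mesh's hit event calls Hit.
; With a valid owner, Hit prints the target's name, ignores itself and the owner, applies damage credited to the owner's instigator controller, plays optional particles and 2D sound, then destroys the projectile.
; Without an owner, it just destroys itself on hit.
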(event `self.ReceiveTick`
  (params (DeltaSeconds :type "Float (single-precision)"))
  (`self.Movement` DeltaSeconds))

(event `self.ProyectilMesh.OnComponentHit`
  (params (HitComponent :type "PrimitiveComponent Object Reference") (OtherActor :type "Actor Object Reference") (OtherComp :type "PrimitiveComponent Object Reference") (NormalImpulse :type "Vector Structure") (Hit :type "HitResult Structure (by ref)"))
  (`self.Hit` OtherActor))

(fn `Hit`
  (params (HitActor :type "Actor Object Reference (by ref)"))
  (locals (MyOwnerInstigator :type "Controller Object Reference"))
  (bind _returnvalue (`self.GetOwner`))
  (bind _hitparticles (`self.HitParticles`))
  (bind _hitsound (`self.HitSound`))
  (`/Engine/EditorBlueprintResources/StandardMacros.IsValid` _returnvalue
    (:`Is Valid`
      (`KismetSystemLibrary.PrintString` (`KismetSystemLibrary.GetDisplayName` HitActor))
      (set `local.MyOwnerInstigator` (`self.GetInstigatorController` _returnvalue))
      (if (and (`KismetSystemLibrary.IsValid` HitActor) (!= HitActor self) (!= HitActor _returnvalue))
        (`GameplayStatics.ApplyDamage` HitActor (`self.Dmg`) (`local.MyOwnerInstigator`) self "/Script/Engine.DamageType")
        (`/Engine/EditorBlueprintResources/StandardMacros.IsValid` _hitparticles
          (:`Is Valid`
            (`GameplayStatics.SpawnEmitterAtLocation` _hitparticles (.location (`self.GetTransform`)) (.rotation (`self.GetTransform`)) (.scale (`self.GetTransform`))))
          (:`Is Not Valid`
            _))
        (`/Engine/EditorBlueprintResources/StandardMacros.IsValid` _hitsound
          (:`Is Valid`
            (`GameplayStatics.SpawnSound2D` _hitsound 1.0 1.0 0.0 null))
          (:`Is Not Valid`
            _))
        (`self.K2_DestroyActor` :!label _label)))
    (:`Is Not Valid`
      (goto _label))))

(fn `Movement`
  (params (DeltaSeconds :type "Float (double-precision) (by ref)"))
  (`self.K2_AddActorLocalOffset` (`KismetMathLibrary.MakeVector` (* DeltaSeconds (`self.Speed`))) true))

(fn `UserConstructionScript`)